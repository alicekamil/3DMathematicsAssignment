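; Target dummy character that reacts physically to hits and supplies an anchor point for impact VFX.
; On BeginPlay it simulates physics on every body below the hip bone, leaving the hip itself out for a partial ragdoll.
; DealDamage pushes those bodies with a directional impulse, scaling intensity up to MaxRagdollStrength.
; GetImpactVFXPosition returns the chest socket location, while ApplyHitForce is an empty stub.
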(event `self.ReceiveBeginPlay`
  (`SkeletalMeshComponent.SetAllBodiesBelowSimulatePhysics` (`self.SkeletalMesh`) "HIpBone" true false))

(event `ApplyHitForce`
  (params (`Impulse Direction` :type "Vector Structure") (ImpulseStrength :type "Float (double-precision)")))

(fn `Deal Damage`
  (params (Direction :type "Vector Structure") (Intensity :type "Float (double-precision)"))
  (`SkeletalMeshComponent.AddImpulseToAllBodiesBelow` (`self.SkeletalMesh`) (* Direction (`KismetMathLibrary.Lerp` 0.0 (`self.Max Ragdoll Strength`) Intensity)) "HIpBone" false true)
  (return))

(fn `Get Impact VFX Position`
  (returns (`Impact VFX Position` :type "Vector Structure"))
  (return (`SceneComponent.GetSocketLocation` (`self.SkeletalMesh`) "ChestBoneB")))

(fn `UserConstructionScript`)