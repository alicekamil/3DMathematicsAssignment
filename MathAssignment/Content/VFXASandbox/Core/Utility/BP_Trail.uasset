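; BP_Trail is an actor that attaches a trail visual effect to its owning actor.
; On BeginPlay it attaches itself to the owner keeping relative transforms, then spawns TrailVFX on its root as either a Niagara system or a Cascade emitter.
; It binds to the owner's destroyed event and destroys itself after an ExtraLifetime delay, so it outlives the owner briefly.
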(event `self.ReceiveBeginPlay`
  (bind _returnvalue (`self.GetOwner`))
  (`|ExecutionSequence`
    (:`then_0`
      (`self.K2_AttachToActor` _returnvalue "None" "KeepRelative" "KeepRelative" "KeepRelative")
      ;[0 0 0 1 45] Spawn Trail VFX
      (bind _asniagara_system (cast `NiagaraSystem` (`self.Trail VFX`))
        (:`then`
          (`NiagaraFunctionLibrary.SpawnSystemAttached` _asniagara_system (`self.DefaultSceneRoot`) "None" (0.0 0.0 0.0) (struct) "KeepRelativeOffset" true))
        (:`CastFailed`
          (bind _asparticle_system (cast `ParticleSystem` (`self.Trail VFX`)))
          (`GameplayStatics.SpawnEmitterAttached` _asparticle_system (`self.DefaultSceneRoot`) "None" (0.0 0.0 0.0) (struct) (1.0 1.0 1.0) "KeepRelativeOffset" false))))
    (:`then_1`
      (add `self.OnDestroyed` _returnvalue (delegate `On Owner Destroyed`)))))

(event `On Owner Destroyed` :!signature `self.OnDestroyed`
  (params (DestroyedActor :type "Actor Object Reference"))
  ;[1 0 0.04483 1 45] When my owner is destroyed, destroy me after the Extra Lifetime
  (`KismetSystemLibrary.Delay` (`self.Extra Lifetime`))
  (`self.K2_DestroyActor`))

(fn `UserConstructionScript`)