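; Character component that manages spell selection and casting in a VFX sandbox.
; On BeginPlay it copies ranged, melee and instant spell definitions from a BP_CreateSpells actor, alongside a custom class-based spellbook.
; StartSpell spawns the selected spell, using Fireball, LightSlash and HealingBurst actors as templates filled with spellbook data.
; Casting is blocked while jumping or while another spell is active; ReleaseSpell releases the active one.
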(event `self.ReceiveBeginPlay`
  ;[0 0 0 1 45] Begin Play - Initialization
  (`|ExecutionSequence`
    (:`then_0`
      (bind _asbp_vfxa_character (cast `/Game/VFXASandbox/Core/Characters/BP_VFXA_Character` (`self.GetOwner`))
        (:`then`
          (set `self.Character` _asbp_vfxa_character))
        (:`CastFailed`
          (`KismetSystemLibrary.PrintString` "SpellcasterComponent added to something that's not a Character"))))
    (:`then_1`
      (`self.Load Spells From CreateSpells`))))

(event `Cycle Next Spell`
  ;[0.3696 0.141 1 1 45] Cycle Selected Spell
  (`/Engine/EditorBlueprintResources/StandardMacros.IncrementInt` (`self.Selected Spell Index`)
    (:`  `
      (`self.Clamp Selected Spell Index`))))

(event `Start Spell`
  ;[0.3696 0.141 1 1 45] Start Spell - Launch the Selected Spell
  (if (`self.Get Can Cast Spell`)
    (bind _spell_spawned_ (`self.Spawn Spell`))
    (`/Engine/EditorBlueprintResources/StandardMacros.IsValid` _spell_spawned_
      (:`Is Valid`
        (`/Game/VFXASandbox/Core/Spells/BP_Spell.Start Spell` (`self.Currently Playing Spell`))))))

(event `Release Spell`
  ;[0.3696 0.141 1 1 45] Release Spell
  (`/Engine/EditorBlueprintResources/StandardMacros.IsValid` (`self.Currently Playing Spell`)
    (:`Is Valid`
      (if (not (`/Game/VFXASandbox/Core/Spells/BP_Spell.bSpellHasReleased` (`self.Currently Playing Spell`)))
        (`/Game/VFXASandbox/Core/Spells/BP_Spell.Release Spell` (`self.Currently Playing Spell`))))))

(fn `Clamp Selected Spell Index`
  (switch `/Game/VFXASandbox/Core/Spells/ESpellType` (`self.Selected Spell Type`)
    (:`NewEnumerator0`
      (set `self.Selected Spell Index` (mod (`self.Selected Spell Index`) (`KismetArrayLibrary.Array_Length` (`self.Spellbook`)))))
    (:`NewEnumerator1`
      (set `self.Selected Spell Index` (mod (`self.Selected Spell Index`) (`KismetArrayLibrary.Array_Length` (`self.Spellbook Ranged`)))))
    (:`NewEnumerator2`
      (set `self.Selected Spell Index` (mod (`self.Selected Spell Index`) (`KismetArrayLibrary.Array_Length` (`self.Spellbook Melee`)))))
    (:`NewEnumerator3`
      (set `self.Selected Spell Index` (mod (`self.Selected Spell Index`) (`KismetArrayLibrary.Array_Length` (`self.Spellbook Instant`))))))
  (return))

(fn `Find Mouse World Location`
  (returns (MouseLocationWorld :type "Vector Structure"))
  (bind (_worldlocation _worlddirection) (`PlayerController.DeprojectMousePositionToWorld` (`GameplayStatics.GetPlayerController` 0)))
  (bind _outhit (`KismetSystemLibrary.LineTraceSingle` _worldlocation (+ _worldlocation (* _worlddirection 9000.0)) "TraceTypeQuery3"))
  (return (`.ImpactPoint` (`GameplayStatics.BreakHitResult` _outhit))))

(fn `Get Can Cast Spell`
  (returns (`Can Cast` :type Boolean))
  (if (not (`/Game/VFXASandbox/Core/Characters/BP_VFXA_Character.Jumping` (`self.Character`)))
    (`/Engine/EditorBlueprintResources/StandardMacros.IsValid` (`self.Currently Playing Spell`)
      (:`Is Valid`
        _)
      (:`Is Not Valid`
        (return true))))
  (return false))

(fn `Get Current Spellbook Size`
  (returns (`Spellbook Size` :type Integer))
  (switch `/Game/VFXASandbox/Core/Spells/ESpellType` (`self.Selected Spell Type`)
    (:`NewEnumerator0`
      (return (`KismetArrayLibrary.Array_Length` (`self.Spellbook`))))
    (:`NewEnumerator1`
      (return (`KismetArrayLibrary.Array_Length` (`self.Spellbook Ranged`))))
    (:`NewEnumerator2`
      (return (`KismetArrayLibrary.Array_Length` (`self.Spellbook Melee`))))
    (:`NewEnumerator3`
      (return (`KismetArrayLibrary.Array_Length` (`self.Spellbook Instant`))))))

(fn `Get Selected Spell`
  (returns (`Selected Spell` :type "/Game/VFXASandbox/Core/Spells/BP_Spell Class Reference"))
  (switch `/Game/VFXASandbox/Core/Spells/ESpellType` (`self.Selected Spell Type`)
    (:`NewEnumerator0`
      (return (`|GetArrayItem` (`self.Spellbook`) (`self.Selected Spell Index`))))
    (:`NewEnumerator1`
      (return "/Game/VFXASandbox/Core/Spells/Default_Spells/Spell_Fireball/BP_Spell_Fireball.BP_Spell_Fireball_C"))
    (:`NewEnumerator2`
      (return "/Game/VFXASandbox/Core/Spells/Default_Spells/Spell_LightSlash/BP_Spell_LightSlash.BP_Spell_LightSlash_C"))
    (:`NewEnumerator3`
      (return "/Game/VFXASandbox/Core/Spells/Default_Spells/Spell_HealingBurst/BP_Spell_HealingBurst.BP_Spell_HealingBurst_C"))))

(fn `Get Selected Spell Icon`
  (returns (`Selected Spell Icon` :type "Texture2D Object Reference"))
  (switch `/Game/VFXASandbox/Core/Spells/ESpellType` (`self.Selected Spell Type`)
    (:`NewEnumerator0`
      (return (`.Spell Icon` (defaults `Object` (`self.Get Selected Spell`)))))
    (:`NewEnumerator1`
      (return "/Game/VFXASandbox/UI/Textures/T_Spell_Ranged.T_Spell_Ranged"))
    (:`NewEnumerator2`
      (return "/Game/VFXASandbox/UI/Textures/T_Spell_Melee.T_Spell_Melee"))
    (:`NewEnumerator3`
      (return "/Game/VFXASandbox/UI/Textures/T_Spell_Instant.T_Spell_Instant"))))

(fn `Get Selected Spell Name`
  (returns (`Selected Spell Name` :type Text))
  (switch `/Game/VFXASandbox/Core/Spells/ESpellType` (`self.Selected Spell Type`)
    (:`NewEnumerator0`
      (return (`.Spell Name` (defaults `Object` (`self.Get Selected Spell`)))))
    (:`NewEnumerator1`
      (return (`.SpellName_20_B1C3D6884543E534BF3DFAB40AEAC341` (break `/Game/VFXASandbox/Core/Spells/SRangedSpellProperties` (`|GetArrayItem` (`self.Spellbook Ranged`) (`self.Selected Spell Index`))))))
    (:`NewEnumerator2`
      (return (`.SpellName_22_A3973DD54186AD5C65913F97CE2605B3` (break `/Game/VFXASandbox/Core/Spells/SMeleeSpellProperties` (`|GetArrayItem` (`self.Spellbook Melee`) (`self.Selected Spell Index`))))))
    (:`NewEnumerator3`
      (return (`.SpellName_26_A4D0271F4C1B030C8EE0F6ABF6815D63` (break `/Game/VFXASandbox/Core/Spells/SInstantSpellProperties` (`|GetArrayItem` (`self.Spellbook Instant`) (`self.Selected Spell Index`))))))))

(fn `Load Spells From CreateSpells`
  (bind _returnvalue (`GameplayStatics.GetActorOfClass` "/Game/VFXASandbox/Core/Spells/BP_CreateSpells.BP_CreateSpells_C"))
  (set `self.Spellbook Ranged` (`/Game/VFXASandbox/Core/Spells/BP_CreateSpells.Ranged Spells` _returnvalue))
  (set `self.Spellbook Melee` (`/Game/VFXASandbox/Core/Spells/BP_CreateSpells.Melee Spells` _returnvalue))
  (set `self.Spellbook Instant` (`/Game/VFXASandbox/Core/Spells/BP_CreateSpells.Instant Spells` _returnvalue)))

(fn `Set SpellType`
  (params (`Spell Type` :type "/Game/VFXASandbox/Core/Spells/ESpellType Enum" :default "NewEnumerator0"))
  (set `self.Selected Spell Type` `Spell Type`)
  (set `self.Selected Spell Index` 0))

(fn `Spawn Spell`
  (returns (`Spell Spawned?` :type "/Game/VFXASandbox/Core/Spells/BP_Spell Object Reference"))
  (switch `/Game/VFXASandbox/Core/Spells/ESpellType` (`self.Selected Spell Type`)
    (:`NewEnumerator0`
      (bind _returnvalue (`|SpawnActorFromClass` (`self.Get Selected Spell`) (`KismetMathLibrary.MakeTransform` (`Actor.K2_GetActorLocation` (`self.Character`))) "Undefined" "SelectDefaultAtRuntime" (`self.Character`) null))
      (bind _output_get (set `self.Currently Playing Spell` _returnvalue))
      (return _output_get))
    (:`NewEnumerator1`
      (bind _spawned (`self.Spawn Spell Ranged`))
      (return _spawned))
    (:`NewEnumerator2`
      (bind _spawned_2 (`self.Spawn Spell Melee`))
      (return _spawned_2))
    (:`NewEnumerator3`
      (bind _spawned_3 (`self.Spawn Spell Instant`))
      (return _spawned_3))))

(fn `Spawn Spell Instant`
  (returns (Spawned :type "/Game/VFXASandbox/Core/Spells/BP_Spell Object Reference"))
  (bind (_output_spellname _output_windupvfx _output_windupvfxsocket _output_castvfx _output_impactvfx _output_areavfx _output_spellmontage _output_impactcollisionradius _output_damageintensity) (break `/Game/VFXASandbox/Core/Spells/SInstantSpellProperties` (`|GetArrayItem` (`self.Spellbook Instant`) (`self.Selected Spell Index`))))
  (if (> (`KismetArrayLibrary.Array_Length` (`self.Spellbook Instant`)) 0)
    (bind _returnvalue (`|SpawnActorFromClass` "/Game/VFXASandbox/Core/Spells/Default_Spells/Spell_HealingBurst/BP_Spell_HealingBurst.BP_Spell_HealingBurst_C" (`KismetMathLibrary.MakeTransform` (`Actor.K2_GetActorLocation` (`self.Character`))) "Undefined" "OverrideRootScale" (`self.Character`) null))
    (set `/Game/VFXASandbox/Core/Spells/BP_Spell.Spell Name` _output_spellname _returnvalue)
    (set `/Game/VFXASandbox/Core/Spells/Default_Spells/Spell_HealingBurst/BP_Spell_HealingBurst.WindUp FX` _output_windupvfx _returnvalue)
    (set `/Game/VFXASandbox/Core/Spells/Default_Spells/Spell_HealingBurst/BP_Spell_HealingBurst.WindUp FX Socket` _output_windupvfxsocket _returnvalue)
    (set `/Game/VFXASandbox/Core/Spells/Default_Spells/Spell_HealingBurst/BP_Spell_HealingBurst.Cast FX` _output_castvfx _returnvalue)
    (set `/Game/VFXASandbox/Core/Spells/Default_Spells/Spell_HealingBurst/BP_Spell_HealingBurst.Area VFX` _output_areavfx _returnvalue)
    (set `/Game/VFXASandbox/Core/Spells/Default_Spells/Spell_HealingBurst/BP_Spell_HealingBurst.Impact VFX` _output_impactvfx _returnvalue)
    (set `/Game/VFXASandbox/Core/Spells/Default_Spells/Spell_HealingBurst/BP_Spell_HealingBurst.Spell Montage` _output_spellmontage _returnvalue)
    (set `/Game/VFXASandbox/Core/Spells/Default_Spells/Spell_HealingBurst/BP_Spell_HealingBurst.Impact Collision Radius` _output_impactcollisionradius _returnvalue)
    (set `/Game/VFXASandbox/Core/Spells/Default_Spells/Spell_HealingBurst/BP_Spell_HealingBurst.Damage Intensity` _output_damageintensity _returnvalue)
    (bind _output_get (set `self.Currently Playing Spell` _returnvalue))
    (return _output_get)
    (else
      (return null))))

(fn `Spawn Spell Melee`
  (returns (Spawned :type "/Game/VFXASandbox/Core/Spells/BP_Spell Object Reference"))
  (bind (_spellname _slashvfx _impactvfx _spellanimationmontage _hurtboxrange _hurtboxwidth _hurtboxheight _hurtboxlifetime _damageintensity) (break `/Game/VFXASandbox/Core/Spells/SMeleeSpellProperties` (`|GetArrayItem` (`self.Spellbook Melee`) (`self.Selected Spell Index`))))
  (if (> (`KismetArrayLibrary.Array_Length` (`self.Spellbook Melee`)) 0)
    (bind _returnvalue (`|SpawnActorFromClass` "/Game/VFXASandbox/Core/Spells/Default_Spells/Spell_LightSlash/BP_Spell_LightSlash.BP_Spell_LightSlash_C" (`KismetMathLibrary.MakeTransform` (`Actor.K2_GetActorLocation` (`self.Character`))) "Undefined" "OverrideRootScale" (`self.Character`) null null))
    (set `/Game/VFXASandbox/Core/Spells/BP_Spell.Spell Name` _spellname _returnvalue)
    (set `/Game/VFXASandbox/Core/Spells/Default_Spells/Spell_LightSlash/BP_Spell_LightSlash.Slash VFX` _slashvfx _returnvalue)
    (set `/Game/VFXASandbox/Core/Spells/Default_Spells/Spell_LightSlash/BP_Spell_LightSlash.Impact VFX` _impactvfx _returnvalue)
    (set `/Game/VFXASandbox/Core/Spells/Default_Spells/Spell_LightSlash/BP_Spell_LightSlash.Spell Montage` _spellanimationmontage _returnvalue)
    (set `/Game/VFXASandbox/Core/Spells/Default_Spells/Spell_LightSlash/BP_Spell_LightSlash.Hurtbox Range` _hurtboxrange _returnvalue)
    (set `/Game/VFXASandbox/Core/Spells/Default_Spells/Spell_LightSlash/BP_Spell_LightSlash.Hurtbox Width` _hurtboxwidth _returnvalue)
    (set `/Game/VFXASandbox/Core/Spells/Default_Spells/Spell_LightSlash/BP_Spell_LightSlash.Hurtbox Height` _hurtboxheight _returnvalue)
    (set `/Game/VFXASandbox/Core/Spells/Default_Spells/Spell_LightSlash/BP_Spell_LightSlash.Hurtbox Lifetime` _hurtboxlifetime _returnvalue)
    (set `/Game/VFXASandbox/Core/Spells/Default_Spells/Spell_LightSlash/BP_Spell_LightSlash.Damage Intensity` _damageintensity _returnvalue)
    (bind _output_get (set `self.Currently Playing Spell` _returnvalue))
    (return _output_get)
    (else
      (return null))))

(fn `Spawn Spell Ranged`
  (returns (Spawned :type "/Game/VFXASandbox/Core/Spells/BP_Spell Object Reference"))
  (bind (_spellname _windupvfx _windupvfxsocket _castvfx _projectileheadvfx _projectiletrailvfx _impactvfx _spellanimationmontage _projectilemaxlifetime _projectilemaxrange _projectilespeed _hurtboxradius _bdestroyonimpact _damageintensity) (break `/Game/VFXASandbox/Core/Spells/SRangedSpellProperties` (`|GetArrayItem` (`self.Spellbook Ranged`) (`self.Selected Spell Index`))))
  (if (> (`KismetArrayLibrary.Array_Length` (`self.Spellbook Ranged`)) 0)
    (bind _returnvalue (`|SpawnActorFromClass` "/Game/VFXASandbox/Core/Spells/Default_Spells/Spell_Fireball/BP_Spell_Fireball.BP_Spell_Fireball_C" (`KismetMathLibrary.MakeTransform` (`Actor.K2_GetActorLocation` (`self.Character`))) "Undefined" "OverrideRootScale" (`self.Character`) null))
    (set `/Game/VFXASandbox/Core/Spells/BP_Spell.Spell Name` _spellname _returnvalue)
    (set `/Game/VFXASandbox/Core/Spells/Default_Spells/Spell_Fireball/BP_Spell_Fireball.WindUp FX` _windupvfx _returnvalue)
    (set `/Game/VFXASandbox/Core/Spells/Default_Spells/Spell_Fireball/BP_Spell_Fireball.WindUp VFX Socket` _windupvfxsocket _returnvalue)
    (set `/Game/VFXASandbox/Core/Spells/Default_Spells/Spell_Fireball/BP_Spell_Fireball.Cast FX` _castvfx _returnvalue)
    (set `/Game/VFXASandbox/Core/Spells/Default_Spells/Spell_Fireball/BP_Spell_Fireball.Projectile Head VFX` _projectileheadvfx _returnvalue)
    (set `/Game/VFXASandbox/Core/Spells/Default_Spells/Spell_Fireball/BP_Spell_Fireball.Projectile Trail VFX` _projectiletrailvfx _returnvalue)
    (set `/Game/VFXASandbox/Core/Spells/Default_Spells/Spell_Fireball/BP_Spell_Fireball.Impact FX` _impactvfx _returnvalue)
    (set `/Game/VFXASandbox/Core/Spells/Default_Spells/Spell_Fireball/BP_Spell_Fireball.Spell Montage` _spellanimationmontage _returnvalue)
    (set `/Game/VFXASandbox/Core/Spells/Default_Spells/Spell_Fireball/BP_Spell_Fireball.Projectile Max Lifetime` _projectilemaxlifetime _returnvalue)
    (set `/Game/VFXASandbox/Core/Spells/Default_Spells/Spell_Fireball/BP_Spell_Fireball.Projectile Max Range` _projectilemaxrange _returnvalue)
    (set `/Game/VFXASandbox/Core/Spells/Default_Spells/Spell_Fireball/BP_Spell_Fireball.Projectile Speed` _projectilespeed _returnvalue)
    (set `/Game/VFXASandbox/Core/Spells/Default_Spells/Spell_Fireball/BP_Spell_Fireball.Hurtbox Radius` _hurtboxradius _returnvalue)
    (set `/Game/VFXASandbox/Core/Spells/Default_Spells/Spell_Fireball/BP_Spell_Fireball.bDestroyOnImpact` _bdestroyonimpact _returnvalue)
    (set `/Game/VFXASandbox/Core/Spells/Default_Spells/Spell_Fireball/BP_Spell_Fireball.Damage Intensity` _damageintensity _returnvalue)
    (bind _output_get (set `self.Currently Playing Spell` _returnvalue))
    (return _output_get)
    (else
      (return null))))