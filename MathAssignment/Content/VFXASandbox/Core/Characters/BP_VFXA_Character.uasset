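; Player character for the VFX sandbox, with camera-relative walk, sprint and jump, and spell start and release forwarded to a spellcaster component.
; Tick projects a world cursor onto the surface under the mouse, updates the AnimBP running flag and smooths spring-arm zoom, compensating for time dilation.
; Camera dragging rotates the view while pinning the mouse at its captured position.
; Helper functions toggle mobility and compute or apply facing toward the cursor.
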(event `self.ReceiveBeginPlay`
  ;[0 0 0 1 45] Begin Play - Initialization
  (bind _asabp_jeanette (cast `/Game/VFXASandbox/Characters/Jeanette_Playable/ABP_Jeanette` (`SkeletalMeshComponent.GetAnimInstance` (`self.Mesh`))))
  (set `self.AnimBP` _asabp_jeanette)
  ;;[0 0 0] This lifts the starting camera position a bit
  (`self.AddControllerPitchInput` 10.0))

(event `Camera Zoom In`
  ;[0.1506 0.5258 1 1 45] Camera Zoom
  (set `self.DesiredCameraDistance` (`KismetMathLibrary.FClamp` (+ (`self.DesiredCameraDistance`) 200.0) (`self.ZoomMin`) (`self.ZoomMax`))))

(event `Camera Zoom Out`
  ;[0.1506 0.5258 1 1 45] Camera Zoom
  (set `self.DesiredCameraDistance` (`KismetMathLibrary.FClamp` (- (`self.DesiredCameraDistance`) 200.0) (`self.ZoomMin`) (`self.ZoomMax`))))

(event `self.ReceiveTick`
  (params (DeltaSeconds :type "Float (single-precision)"))
  (bind _desiredcameradistance (`self.DesiredCameraDistance`))
  (bind _targetarmlength (`SpringArmComponent.TargetArmLength` (`self.Camera Crane`)))
  (bind (_bblockinghit _binitialoverlap _time _distance _location _impactpoint _normal _impactnormal) (`GameplayStatics.BreakHitResult` (`PlayerController.GetHitResultUnderCursorByChannel` (`GameplayStatics.GetPlayerController` 0) "TraceTypeQuery1" true)))
  (set `self.Delta Seconds` DeltaSeconds)
  (`|ExecutionSequence`
    (:`then_0`
      ;[0 0 0 1 45] Check if the character has finished jumping
      (if (and (`NavMovementComponent.IsMovingOnGround` (`self.CharacterMovement`)) (`self.Jumping`))
        (set `self.Jumping` false)))
    (:`then_1`
      ;[0 0 0 1 45] Cursor
      (`SceneComponent.K2_SetWorldLocationAndRotation` (`self.CursorToWorld`) _location (`KismetMathLibrary.MakeRotationFromAxes` _impactnormal) false false))
    (:`then_2`
      ;[0 0 0 1 45] Update AnimBP Variables
      (set `/Game/VFXASandbox/Characters/Jeanette_Playable/ABP_Jeanette.Running?` (> (`KismetMathLibrary.VSize` (`MovementComponent.Velocity` (`self.CharacterMovement`))) 10.0) (`self.AnimBP`)))
    (:`then_3`
      ;[0 0 0 1 45] Capture mouse while moving the camera
      (if (`self.bIsCameraMoving`)
        (`PlayerController.SetMouseLocation` (`GameplayStatics.GetPlayerController` 0) (`self.CapturedMousePositionX`) (`self.CapturedMousePositionY`))))
    (:`then_4`
      ;[0 0 0 1 45] SpringArm Lerping
      (if (> (`KismetMathLibrary.Abs` (- _targetarmlength _desiredcameradistance)) 1.0)
        (set `SpringArmComponent.TargetArmLength` (`KismetMathLibrary.Lerp` _targetarmlength _desiredcameradistance (`KismetMathLibrary.FClamp` (/ (* (`self.Delta Seconds`) (`self.Camera Zoom Speed`)) (`GameplayStatics.GetGlobalTimeDilation`)))) (`self.Camera Crane`))))))

(event `Camera Drag Start`
  (bind (_locationx _locationy) (`PlayerController.GetMousePosition` (`GameplayStatics.GetPlayerController` 0)))
  ;[0.1506 0.5258 1 1 45] Camera Rotation
  (set `self.bIsCameraMoving` true)
  (set `self.CapturedMousePositionX` (`KismetMathLibrary.FTrunc` _locationx))
  (set `self.CapturedMousePositionY` (`KismetMathLibrary.FTrunc` _locationy)))

(event `Camera Drag End`
  ;[0.1506 0.5258 1 1 45] Camera Rotation
  (set `self.bIsCameraMoving` false))

(event `InputAxisKey|MouseX`
  (params (AxisValue :type "Float (single-precision)"))
  ;[0.1506 0.5258 1 1 45] Camera Rotation
  (if (`self.bIsCameraMoving`)
    (`self.AddControllerYawInput` AxisValue)))

(event `InputAxisKey|MouseY`
  (params (AxisValue :type "Float (single-precision)"))
  ;[0.1506 0.5258 1 1 45] Camera Rotation
  (if (`self.bIsCameraMoving`)
    (`self.AddControllerPitchInput` (* AxisValue -1.0))))

(event `Start Spell`
  ;[0.3696 0.141 1 1 45] Launch Spells
  (`/Game/VFXASandbox/Core/Characters/BP_SpellcasterComponent.Start Spell` (`self.BP_SpellcasterComponent`)))

(event `Release Spell`
  ;[0.3696 0.141 1 1 45] Launch Spells
  (`/Game/VFXASandbox/Core/Characters/BP_SpellcasterComponent.Release Spell` (`self.BP_SpellcasterComponent`)))

(event `InputAxis|MoveForward`
  (params (AxisValue :type "Float (single-precision)"))
  ;[0.3237 1 0.2637 1 45] Character Movement - Walk
  (if (`self.CanMove`)
    (`self.AddMovementInput` (`KismetMathLibrary.GetForwardVector` (`KismetMathLibrary.MakeRotator` 0.0 0.0 (.yaw (`Controller.GetControlRotation` (`GameplayStatics.GetPlayerController` 0))))) AxisValue)))

(event `InputAxis|MoveRight`
  (params (AxisValue :type "Float (single-precision)"))
  ;[0.3237 1 0.2637 1 45] Character Movement - Walk
  (if (`self.CanMove`)
    (`self.AddMovementInput` (`KismetMathLibrary.GetRightVector` (`KismetMathLibrary.MakeRotator` 0.0 0.0 (.yaw (`Controller.GetControlRotation` (`GameplayStatics.GetPlayerController` 0))))) AxisValue)))

(event `InputAction|Sprint`
  (params (Key :type "Key Structure"))
  ;[0.3237 1 0.2637 1 45] Character Movement - Sprint
  (:`Pressed`
    (set `self.Running` true)
    (set `CharacterMovementComponent.MaxWalkSpeed` (`self.sprintSpeed`) (`self.CharacterMovement`)))
  (:`Released`
    (set `self.Running` false)
    (set `CharacterMovementComponent.MaxWalkSpeed` (`self.walkSpeed`) (`self.CharacterMovement`))))

(event `InputAction|Jump`
  (params (Key :type "Key Structure"))
  ;[0.3237 1 0.2637 1 45] Character Movement - Jump
  (:`Pressed`
    (if (and (`NavMovementComponent.IsMovingOnGround` (`self.CharacterMovement`)) (`self.CanMove`) (not (`self.Jumping`)))
      (set `self.Jumping` true)
      (`self.Jump`))))

(fn `Get LookAtCursor Rotation`
  (returns (`LookAt Rotation` :type "Rotator Structure"))
  (return (`KismetMathLibrary.FindLookAtRotation` (* (`SceneComponent.K2_GetComponentLocation` (`self.CapsuleComponent`)) (1.0 1.0 0.0)) (* (`SceneComponent.K2_GetComponentLocation` (`self.CursorToWorld`)) (1.0 1.0 0.0)))))

(fn `Load Spells from CreateSpells`)

(fn `LookAtCursor`
  (`self.K2_SetActorRotation` (`KismetMathLibrary.FindLookAtRotation` (* (`SceneComponent.K2_GetComponentLocation` (`self.CapsuleComponent`)) (1.0 1.0 0.0)) (* (`SceneComponent.K2_GetComponentLocation` (`self.CursorToWorld`)) (1.0 1.0 0.0))) true)
  (return))

(fn `Set Character Mobility`
  (params (`Can Move` :type Boolean) (`Orient Rotation To Movement` :type Boolean))
  (set `self.CanMove` `Can Move`)
  (set `CharacterMovementComponent.bOrientRotationToMovement` `Orient Rotation To Movement` (`self.CharacterMovement`)))

(fn `UserConstructionScript`)