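; Fireball spell Blueprint that roots the caster, plays a wind-up and cast montage, and launches a fireball projectile.
; Start and release turn the caster to the cursor (optionally tracked while holding) and switch montage sections; release restores movement and destroys the spell after a delay.
; SpellEvent01 attaches wind-up VFX; SpellEvent02 spawns cast VFX and the configured projectile, then removes the wind-up.
; VFX helpers accept either Cascade or Niagara systems.
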(event `self.ReceiveBeginPlay`
  ;[0 0 0 1 45] Begin Play
  (`parent.ReceiveBeginPlay`))

(event `self.ReceiveTick`
  (params (DeltaSeconds :type "Float (single-precision)"))
  ;[0 0 0 1 45] Tick - If requested, look at the cursor while holding the spell windUp
  (`parent.ReceiveTick` DeltaSeconds)
  (if (`self.bLookAtCursorWhileHolding`)
    (if (and (`self.bSpellHasStarted`) (not (`self.bSpellHasReleased`)))
      (`/Game/VFXASandbox/Core/Characters/BP_VFXA_Character.LookAtCursor` (`self.Caster Character`)))))

(event `self.Start Spell`
  ;[0 0 0 1 45] Start Spell - Look at cursor, play the spell animation and make the caster immobile
  (`parent.Start Spell`)
  (`/Game/VFXASandbox/Core/Characters/BP_VFXA_Character.LookAtCursor` (`self.Caster Character`))
  (`/Game/VFXASandbox/Characters/Jeanette_Playable/ABP_Jeanette.Play Montage` (`/Game/VFXASandbox/Core/Characters/BP_VFXA_Character.AnimBP` (`self.Caster Character`)) (`self.Spell Montage`) "Default" self)
  (`/Game/VFXASandbox/Core/Characters/BP_VFXA_Character.Set Character Mobility` (`self.Caster Character`) false false))

(event `self.Release Spell`
  ;[0 0 0 1 45] Release Spell - Look at cursor, jump to the "Cast" section of the animation, let the caster move and destroy spell
  (`parent.Release Spell`)
  (`/Game/VFXASandbox/Core/Characters/BP_VFXA_Character.LookAtCursor` (`self.Caster Character`))
  (`/Game/VFXASandbox/Characters/Jeanette_Playable/ABP_Jeanette.Play Montage` (`/Game/VFXASandbox/Core/Characters/BP_VFXA_Character.AnimBP` (`self.Caster Character`)) (`self.Spell Montage`) "Cast" self)
  (`KismetSystemLibrary.Delay` 0.66)
  (`/Game/VFXASandbox/Core/Characters/BP_VFXA_Character.Set Character Mobility` (`self.Caster Character`) true true)
  (`self.K2_DestroyActor`))

(event `self.On Spell Event 01`
  ;[0.3696 0.141 1 1 45] On SpellEvent 01- Attach to character and spawn WindUp particles
  (`parent.On Spell Event 01`)
  (`self.K2_AttachToComponent` (`Character.Mesh` (`self.Caster Character`)) (`self.WindUp VFX Socket`) "SnapToTarget" "KeepRelative" "KeepRelative")
  (`self.Spawn WindUp Particles`))

(event `self.On Spell Event 02`
  (bind _caster_character (`self.Caster Character`))
  (bind _returnvalue (`self.K2_GetActorRotation` _caster_character))
  (bind _returnvalue_2 (`SceneComponent.GetSocketLocation` (`Character.Mesh` _caster_character) "CastSocket"))
  ;[0.3696 0.141 1 1 45] On SpellEvent 02 -  Spawn the Fireball Projectile, remove the WindUp
  (`parent.On Spell Event 02`)
  (`self.Spawn Cast Particles` _returnvalue_2 _returnvalue)
  (`|SpawnActorFromClass` "/Game/VFXASandbox/Core/Spells/Default_Spells/Spell_Fireball/BP_Spell_Fireball_Projectile.BP_Spell_Fireball_Projectile_C" (`KismetMathLibrary.MakeTransform` _returnvalue_2 _returnvalue) "Undefined" "OverrideRootScale" null (`KismetMathLibrary.MakeVector` (`self.Projectile Speed`)) (`self.Projectile Max Lifetime`) (`self.Projectile Max Range`) (`self.bDestroyOnImpact`) (`self.Hurtbox Radius`) (`self.Damage Intensity`) (`self.Projectile Head VFX`) (`self.Projectile Trail VFX`) (`self.Impact FX`) null)
  (`self.Stop WindUp Particles`))

(fn `Spawn Cast Particles`
  (params (Location :type "Vector Structure") (Rotation :type "Rotator Structure"))
  (bind _asparticle_system (cast `ParticleSystem` (`self.Cast FX`))
    (:`then`
      (`GameplayStatics.SpawnEmitterAtLocation` _asparticle_system Location Rotation))
    (:`CastFailed`
      (`NiagaraFunctionLibrary.SpawnSystemAtLocation` (cast `NiagaraSystem` (`self.Cast FX`) :!pure true) Location Rotation))))

(fn `Spawn WindUp Particles`
  (bind _asparticle_system (cast `ParticleSystem` (`self.WindUp FX`))
    (:`then`
      (bind _returnvalue (`GameplayStatics.SpawnEmitterAttached` _asparticle_system (`self.DefaultSceneRoot`)))
      (set `self.WindUp Particles` _returnvalue))
    (:`CastFailed`
      (bind _asniagara_system (cast `NiagaraSystem` (`self.WindUp FX`)))
      (bind _returnvalue_2 (`NiagaraFunctionLibrary.SpawnSystemAttached` _asniagara_system (`self.DefaultSceneRoot`) "None" (0.0 0.0 0.0) (struct) "KeepRelativeOffset" true))
      (set `self.WindUp Particles` _returnvalue_2))))

(fn `Stop WindUp Particles`
  (bind _windup_particles (`self.WindUp Particles`))
  (`/Engine/EditorBlueprintResources/StandardMacros.IsValid` _windup_particles
    (:`Is Valid`
      (`ActorComponent.K2_DestroyComponent` _windup_particles)
      (return))))

(fn `UserConstructionScript`
  (`parent.UserConstructionScript`))