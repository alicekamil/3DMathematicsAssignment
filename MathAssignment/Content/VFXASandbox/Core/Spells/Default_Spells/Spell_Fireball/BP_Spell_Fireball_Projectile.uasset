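; Fireball spell projectile that flies forward, damages enemies it overlaps and is destroyed on impact (optional), past a max range or after a lifetime timer.
; BeginPlay sizes the hurtbox, attaches the head VFX and launches local-space velocity.
; Overlaps call BPI_Enemy DealDamage with direction and intensity, then spawn impact VFX at the enemy-provided position.
; Head and impact effects accept Cascade or Niagara; a separate BP_Trail actor keeps the trail from ending abruptly.
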(event `self.ReceiveBeginPlay`
  ;[0 0 0 1 45] Begin Play - Initialization and spawning of the projectile
  (`|ExecutionSequence`
    (:`then_0`
      ;;[0 0 0] Set Collider Size
      (`SphereComponent.SetSphereRadius` (`self.Hurtbox Collider`) (`self.Hurtbox Radius`) true)
      ;;[0 0 0] Remember the initial location
      (set `self.StartLocation` (`self.K2_GetActorLocation`)))
    (:`then_1`
      (`self.Spawn Projectile VFX`)
      (`ProjectileMovementComponent.SetVelocityInLocalSpace` (`self.ProjectileMovement`) (`self.Projectile Velocity`))
      (`KismetSystemLibrary.K2_SetTimerDelegate` (delegate `DestroyActor`) (`self.Projectile Max Lifetime`)))))

(event `DestroyActor`
  (bind _missile_fx (`self.Missile_FX`))
  ;[1 0.05208 0.0653 1 45] Destroy Actor
  (`/Engine/EditorBlueprintResources/StandardMacros.IsValid` _missile_fx
    (:`Is Valid`
      (`ActorComponent.Deactivate` _missile_fx)
      (`self.K2_DestroyActor`))))

(event `self.ReceiveTick`
  (params (DeltaSeconds :type "Float (single-precision)"))
  ;[0 0 0 1 45] Tick - Executed every frame
  (if (> (`self.Projectile Max Range`) 0.0)
    (if (> (`KismetMathLibrary.Vector_Distance` (`self.StartLocation`) (`self.K2_GetActorLocation`)) (`self.Projectile Max Range`))
      (`self.K2_DestroyActor`))))

(event `self.Hurtbox Collider.OnComponentBeginOverlap`
  (params (OverlappedComponent :type "PrimitiveComponent Object Reference") (OtherActor :type "Actor Object Reference") (OtherComp :type "PrimitiveComponent Object Reference") (OtherBodyIndex :type Integer) (bFromSweep :type Boolean) (SweepResult :type "HitResult Structure (by ref)"))
  ;[0 0 0 1 45] On Collision, Spawn FX and apply physics force
  (bind _asbpi_enemy (cast `/Game/VFXASandbox/Core/Characters/BPI_Enemy` OtherActor))
  (`/Game/VFXASandbox/Core/Characters/BPI_Enemy.Deal Damage` _asbpi_enemy (`KismetMathLibrary.GetDirectionUnitVector` (`self.K2_GetActorLocation`) (`SceneComponent.K2_GetComponentLocation` OtherComp)) (`self.Damage Intensity`))
  (bind _impact_vfx_position (`/Game/VFXASandbox/Core/Characters/BPI_Enemy.Get Impact VFX Position` _asbpi_enemy))
  (`self.Spawn Impact VFX` _impact_vfx_position)
  (if (`self.Destroy on Impact?`)
    (`self.K2_DestroyActor`)))

(fn `Spawn Impact VFX`
  (params (Location :type "Vector Structure"))
  (bind _asparticle_system (cast `ParticleSystem` (`self.Impact FX`))
    (:`then`
      (`GameplayStatics.SpawnEmitterAtLocation` _asparticle_system Location))
    (:`CastFailed`
      (`NiagaraFunctionLibrary.SpawnSystemAtLocation` (cast `NiagaraSystem` (`self.Impact FX`) :!pure true) Location))))

(fn `Spawn Projectile VFX`
  (`|ExecutionSequence`
    (:`then_0`
      ;[0.3696 0.141 1 1 45] Spawn Projectile Head particles attached to the projectile
      (bind _asparticle_system (cast `ParticleSystem` (`self.Projectile Head VFX`))
        (:`then`
          (bind _returnvalue (`GameplayStatics.SpawnEmitterAttached` _asparticle_system (`self.RootComponent`) "None" (0.0 0.0 0.0) (struct) (1.0 1.0 1.0) "SnapToTarget"))
          (set `self.Missile_FX` _returnvalue))
        (:`CastFailed`
          (bind _returnvalue_2 (`NiagaraFunctionLibrary.SpawnSystemAttached` (cast `NiagaraSystem` (`self.Projectile Head VFX`) :!pure true) (`self.RootComponent`) "None" (0.0 0.0 0.0) (struct) "SnapToTarget" true))
          (set `self.Missile_FX` _returnvalue_2))))
    (:`then_1`
      ;[0.3696 0.141 1 1 45] Spawn a BP_Trail that handles the Projectile Trail VFX so it doesn't end abruptly when the projectile is destroyed
      (`|SpawnActorFromClass` "/Game/VFXASandbox/Core/Utility/BP_Trail.BP_Trail_C" (`KismetMathLibrary.MakeTransform` (0.0 0.0 0.0)) "Undefined" "OverrideRootScale" self 1.5 (`self.Projectile Trail VFX`) null))))

(fn `UserConstructionScript`)