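; Area actor for the Healing Burst spell that, despite its name, damages enemies entering its radius.
; On BeginPlay it spawns the area effect, sizes the hurtbox sphere and starts a self-destruct timer.
; Overlapped BPI_Enemy actors take directional damage and trigger an impact effect at their reported position.
; Both effects accept Niagara or Cascade assets and attach to the actor's root at world positions.
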(event `self.ReceiveBeginPlay`
  ;[0 0 0 1 45] Begin Play
  (`self.Spawn Area VFX`)
  (`SphereComponent.SetSphereRadius` (`self.Hurtbox Collider`) (`self.Impact Detection Radius`) true)
  (`KismetSystemLibrary.K2_SetTimerDelegate` (delegate `Selfdestruct`) (`self.Lifetime`)))

(event `Selfdestruct`
  ;[0.5312 0 0 1 45] Self Destruct
  (set `PrimitiveComponent.bGenerateOverlapEvents` false (`self.Hurtbox Collider`))
  (`self.K2_DestroyActor`))

(event `self.Hurtbox Collider.OnComponentBeginOverlap`
  (params (OverlappedComponent :type "PrimitiveComponent Object Reference") (OtherActor :type "Actor Object Reference") (OtherComp :type "PrimitiveComponent Object Reference") (OtherBodyIndex :type Integer) (bFromSweep :type Boolean) (SweepResult :type "HitResult Structure (by ref)"))
  ;[0 0 0 1 45] Spawn Hit Impact on Enemies
  (bind _asbpi_enemy (cast `/Game/VFXASandbox/Core/Characters/BPI_Enemy` OtherActor))
  (`/Game/VFXASandbox/Core/Characters/BPI_Enemy.Deal Damage` _asbpi_enemy (`KismetMathLibrary.GetDirectionUnitVector` (`self.K2_GetActorLocation`) (`self.K2_GetActorLocation` OtherActor)) (`self.Damage Intensity`))
  (bind _impact_vfx_position (`/Game/VFXASandbox/Core/Characters/BPI_Enemy.Get Impact VFX Position` _asbpi_enemy))
  (`self.Spawn Impact VFX` _impact_vfx_position))

(fn `Spawn Area VFX`
  (bind _area_fx (`self.Area FX`))
  (`/Engine/EditorBlueprintResources/StandardMacros.IsValid` (`self.Area FX`)
    (:`Is Valid`
      (bind _asniagara_system (cast `NiagaraSystem` _area_fx)
        (:`then`
          (bind _returnvalue (`NiagaraFunctionLibrary.SpawnSystemAttached` _asniagara_system (`self.DefaultSceneRoot`) "None" (`self.K2_GetActorLocation`) (struct) "KeepWorldPosition" true))
          (set `self.SpawnFXNiagara` _returnvalue))
        (:`CastFailed`
          (bind _asparticle_system (cast `ParticleSystem` _area_fx))
          (bind _returnvalue_2 (`GameplayStatics.SpawnEmitterAttached` _asparticle_system (`self.DefaultSceneRoot`) "None" (`self.K2_GetActorLocation`) (struct) (1.0 1.0 1.0) "KeepWorldPosition"))
          (set `self.SpawnFX` _returnvalue_2))))))

(fn `Spawn Impact VFX`
  (params (Location :type "Vector Structure"))
  (bind _asniagara_system (cast `NiagaraSystem` (`self.Impact FX`))
    (:`then`
      (`NiagaraFunctionLibrary.SpawnSystemAttached` _asniagara_system (`self.DefaultSceneRoot`) "None" Location (struct) "KeepWorldPosition" true))
    (:`CastFailed`
      (`GameplayStatics.SpawnEmitterAttached` (cast `ParticleSystem` (`self.Impact FX`) :!pure true) (`self.DefaultSceneRoot`) "None" Location (struct) (1.0 1.0 1.0) "KeepWorldPosition"))))

(fn `UserConstructionScript`)