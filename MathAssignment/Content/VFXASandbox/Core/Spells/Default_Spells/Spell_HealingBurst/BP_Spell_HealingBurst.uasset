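; Healing Burst spell actor that drops a healing area at the mouse cursor's world position.
; Start and release play montage sections, locking the caster's movement until shortly after release, when the spell destroys itself.
; Spell events attach wind-up VFX to the caster, then swap it for cast VFX and spawn BP_Spell_HealingBurst_Area at a cursor line-trace hit.
; Effect slots accept either Cascade or Niagara systems.
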(event `self.ReceiveBeginPlay`
  ;[0 0 0 1 45] Begin Play
  (`parent.ReceiveBeginPlay`))

(event `self.ReceiveTick`
  (params (DeltaSeconds :type "Float (single-precision)"))
  ;[0 0 0 1 45] Tick - If requested, look at the cursor while holding the spell windUp
  (`parent.ReceiveTick` DeltaSeconds)
  (if (`self.bLookAtCursorWhileHolding`)
    (if (and (`self.bSpellHasStarted`) (not (`self.bSpellHasReleased`)))
      (`/Game/VFXASandbox/Core/Characters/BP_VFXA_Character.LookAtCursor` (`self.Caster Character`)))))

(event `self.Start Spell`
  ;[0 0 0 1 45] Start Spell - Play Animation and make caster immobile
  (`parent.Start Spell`)
  (`/Game/VFXASandbox/Characters/Jeanette_Playable/ABP_Jeanette.Play Montage` (`/Game/VFXASandbox/Core/Characters/BP_VFXA_Character.AnimBP` (`self.Caster Character`)) (`self.Spell Montage`) "Default" self)
  (`/Game/VFXASandbox/Core/Characters/BP_VFXA_Character.Set Character Mobility` (`self.Caster Character`) false false)
  (`/Game/VFXASandbox/Core/Characters/BP_VFXA_Character.LookAtCursor` (`self.Caster Character`)))

(event `self.Release Spell`
  ;[0 0 0 1 45] Release Spell - Let the caster move again
  (`parent.Release Spell`)
  (`/Game/VFXASandbox/Characters/Jeanette_Playable/ABP_Jeanette.Play Montage` (`/Game/VFXASandbox/Core/Characters/BP_VFXA_Character.AnimBP` (`self.Caster Character`)) (`self.Spell Montage`) "Cast" self)
  (`KismetSystemLibrary.Delay` 1.5)
  (`/Game/VFXASandbox/Core/Characters/BP_VFXA_Character.Set Character Mobility` (`self.Caster Character`) true true)
  (`self.K2_DestroyActor`))

(event `self.On Spell Event 01`
  ;[0.3696 0.141 1 1 45] On SpellEvent 01- Attach to character and spawn WindUp particles
  (`parent.On Spell Event 01`)
  (`self.K2_AttachToComponent` (`Character.Mesh` (`self.Caster Character`)) (`self.WindUp FX Socket`) "SnapToTarget" "KeepRelative" "KeepRelative")
  (`self.Spawn WindUp VFX`))

(event `self.On Spell Event 02`
  (bind _windup_vfx_component (`self.WindUp VFX Component`))
  ;[0.3696 0.141 1 1 45] On SpellEvent 02 -  Stop the WindUp VFX and spawn the healing area actor
  (`parent.On Spell Event 02`)
  (`/Engine/EditorBlueprintResources/StandardMacros.IsValid` _windup_vfx_component
    (:`Is Valid`
      (`ActorComponent.K2_DestroyComponent` _windup_vfx_component))
    (:`Is Not Valid`
      _))
  (`self.Spawn Cast VFX`)
  (bind _mouselocationworld (`self.Find Mouse World Location`))
  (`|SpawnActorFromClass` "/Game/VFXASandbox/Core/Spells/Default_Spells/Spell_HealingBurst/BP_Spell_HealingBurst_Area.BP_Spell_HealingBurst_Area_C" (`KismetMathLibrary.MakeTransform` (`KismetMathLibrary.MakeVector` (.x _mouselocationworld) (.y _mouselocationworld) (.z _mouselocationworld))) "Undefined" "OverrideRootScale" null (`self.Impact Collision Radius`) (`self.Damage Intensity`) (`self.Impact VFX`) (`self.Area VFX`) null))

(fn `Find Mouse World Location`
  (returns (MouseLocationWorld :type "Vector Structure"))
  (bind (_worldlocation _worlddirection) (`PlayerController.DeprojectMousePositionToWorld` (`GameplayStatics.GetPlayerController` 0)))
  (bind _outhit (`KismetSystemLibrary.LineTraceSingle` _worldlocation (+ _worldlocation (* _worlddirection 9000.0)) "TraceTypeQuery3"))
  (return (`.ImpactPoint` (`GameplayStatics.BreakHitResult` _outhit))))

(fn `Spawn Cast VFX`
  (bind _mesh (`Character.Mesh` (`self.Caster Character`)))
  (bind _mesh_2 (`Character.Mesh` (`self.Caster Character`)))
  (bind _asparticle_system (cast `ParticleSystem` (`self.Cast FX`))
    (:`then`
      (bind _returnvalue (`GameplayStatics.SpawnEmitterAttached` _asparticle_system (`self.DefaultSceneRoot`)))
      (`SceneComponent.K2_AttachToComponent` _returnvalue _mesh_2 (`SkinnedMeshComponent.GetSocketBoneName` _mesh_2 "CastSocket") "SnapToTarget" "KeepRelative" "KeepRelative" true))
    (:`CastFailed`
      (bind _asniagara_system (cast `NiagaraSystem` (`self.Cast FX`)))
      (bind _returnvalue_2 (`NiagaraFunctionLibrary.SpawnSystemAttached` _asniagara_system (`self.DefaultSceneRoot`) "None" (0.0 0.0 0.0) (struct) "KeepRelativeOffset" true))
      (`SceneComponent.K2_AttachToComponent` _returnvalue_2 _mesh (`SkinnedMeshComponent.GetSocketBoneName` _mesh "CastSocket") "SnapToTarget" "KeepRelative" "KeepRelative" true))))

(fn `Spawn WindUp VFX`
  (bind _asparticle_system (cast `ParticleSystem` (`self.WindUp FX`))
    (:`then`
      (bind _returnvalue (`GameplayStatics.SpawnEmitterAttached` _asparticle_system (`self.DefaultSceneRoot`)))
      (set `self.WindUp VFX Component` _returnvalue))
    (:`CastFailed`
      (bind _asniagara_system (cast `NiagaraSystem` (`self.WindUp FX`)))
      (bind _returnvalue_2 (`NiagaraFunctionLibrary.SpawnSystemAttached` _asniagara_system (`self.DefaultSceneRoot`) "None" (0.0 0.0 0.0) (struct) "KeepRelativeOffset" true))
      (set `self.WindUp VFX Component` _returnvalue_2))))

(fn `UserConstructionScript`
  (`parent.UserConstructionScript`))