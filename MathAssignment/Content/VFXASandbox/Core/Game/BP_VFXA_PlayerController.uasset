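; Player controller for the VFX sandbox that turns keyboard and mouse input into spell, camera and presentation controls.
; On BeginPlay it caches the player's BP_VFXA_Character, shows the cursor and creates the main UI plus a hidden-UI widget.
; Spell selection goes to the character's spellcaster component, while casting, zoom and camera drag go to the character.
; It also toggles UI, cursor and character mesh visibility, and steps or resets clamped global time dilation.
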(event `self.ReceiveBeginPlay`
  ;[0 0 0 1 45] Begin Play - Initialize
  (`|ExecutionSequence`
    (:`then_0`
      ;;[0 0 0] Save Character Reference
      (bind _asbp_vfxa_character (cast `/Game/VFXASandbox/Core/Characters/BP_VFXA_Character` (`GameplayStatics.GetPlayerPawn` 0)))
      (set `self.Character Controller` _asbp_vfxa_character))
    (:`then_1`
      ;;[0 0 0] Setup Cursor
      (set `self.bShowMouseCursor` true))
    (:`then_2`
      (`self.Setup UI`))))

(event `Key|Tab`
  (params (Key :type "Key Structure"))
  ;[0.3696 0.141 1 1 45] Input Handling - Spells
  (:`Pressed`
    (`/Game/VFXASandbox/Core/Characters/BP_SpellcasterComponent.Cycle Next Spell` (`/Game/VFXASandbox/Core/Characters/BP_VFXA_Character.BP_SpellcasterComponent` (`self.Character Controller`)))))

(event `InputAction|MouseWheelDown`
  (params (Key :type "Key Structure"))
  ;[0.1506 0.5258 1 1 45] Input Handling - Camera Zoom
  (:`Pressed`
    (`/Game/VFXASandbox/Core/Characters/BP_VFXA_Character.Camera Zoom In` (`self.Character Controller`))))

(event `InputAction|HideUI`
  (params (Key :type "Key Structure"))
  (bind _ui_widget (`self.UI Widget`))
  (bind _hidden_ui_widget (`self.Hidden UI Widget`))
  ;[0.1506 0.5258 1 1 45] Input Handling - UI
  (:`Pressed`
    (if (`Widget.IsVisible` (`self.UI Widget`))
      (`Widget.SetVisibility` _ui_widget "Hidden")
      (`Widget.SetVisibility` _hidden_ui_widget "Visible")
      (else
        (`Widget.SetVisibility` _ui_widget "Visible")
        (`Widget.SetVisibility` _hidden_ui_widget "Hidden")))))

(event `Key|LeftMouseButton`
  (params (Key :type "Key Structure"))
  ;[0.3696 0.141 1 1 45] Input Handling - Spells
  (:`Pressed`
    (`/Game/VFXASandbox/Core/Characters/BP_VFXA_Character.Start Spell` (`self.Character Controller`)))
  (:`Released`
    (`/Game/VFXASandbox/Core/Characters/BP_VFXA_Character.Release Spell` (`self.Character Controller`))))

(event `InputAction|MouseWheelUp`
  (params (Key :type "Key Structure"))
  ;[0.1506 0.5258 1 1 45] Input Handling - Camera Zoom
  (:`Pressed`
    (`/Game/VFXASandbox/Core/Characters/BP_VFXA_Character.Camera Zoom Out` (`self.Character Controller`))))

(event `Key|One`
  (params (Key :type "Key Structure"))
  ;[0.3696 0.141 1 1 45] Input Handling - Spells
  (:`Pressed`
    (`/Game/VFXASandbox/Core/Characters/BP_SpellcasterComponent.Set SpellType` (`/Game/VFXASandbox/Core/Characters/BP_VFXA_Character.BP_SpellcasterComponent` (`self.Character Controller`)) "NewEnumerator1")))

(event `InputAction|HideChar`
  (params (Key :type "Key Structure"))
  ;[0.1506 0.5258 1 1 45] Input Handling - Character and Cursor visibility
  (:`Pressed`
    (bind _output_get (set `self.bIsCharacterVisible` (not (`self.bIsCharacterVisible`))))
    (`SceneComponent.SetVisibility` (`Character.Mesh` (`self.Character Controller`)) _output_get false)))

(event `InputAction|MoveCam`
  (params (Key :type "Key Structure"))
  (bind _character_controller (`self.Character Controller`))
  ;[0.1506 0.5258 1 1 45] Input Handling - Camera Drag
  (:`Pressed`
    (`/Game/VFXASandbox/Core/Characters/BP_VFXA_Character.Camera Drag Start` _character_controller))
  (:`Released`
    (`/Game/VFXASandbox/Core/Characters/BP_VFXA_Character.Camera Drag End` _character_controller)))

(event `Key|Two`
  (params (Key :type "Key Structure"))
  ;[0.3696 0.141 1 1 45] Input Handling - Spells
  (:`Pressed`
    (`/Game/VFXASandbox/Core/Characters/BP_SpellcasterComponent.Set SpellType` (`/Game/VFXASandbox/Core/Characters/BP_VFXA_Character.BP_SpellcasterComponent` (`self.Character Controller`)) "NewEnumerator2")))

(event `InputAction|HideCursor`
  (params (Key :type "Key Structure"))
  ;[0.1506 0.5258 1 1 45] Input Handling - Character and Cursor visibility
  (:`Pressed`
    (set `self.bShowMouseCursor` (not (`self.bShowMouseCursor`)))
    (`self.Refresh Mouse Position`)))

(event `Key|Three`
  (params (Key :type "Key Structure"))
  ;[0.3696 0.141 1 1 45] Input Handling - Spells
  (:`Pressed`
    (`/Game/VFXASandbox/Core/Characters/BP_SpellcasterComponent.Set SpellType` (`/Game/VFXASandbox/Core/Characters/BP_VFXA_Character.BP_SpellcasterComponent` (`self.Character Controller`)) "NewEnumerator3")))

(event `Key|Four`
  (params (Key :type "Key Structure"))
  ;[0.3696 0.141 1 1 45] Input Handling - Spells
  (:`Pressed`
    (`/Game/VFXASandbox/Core/Characters/BP_SpellcasterComponent.Set SpellType` (`/Game/VFXASandbox/Core/Characters/BP_VFXA_Character.BP_SpellcasterComponent` (`self.Character Controller`)) "NewEnumerator0")))

(event `InputAction|TimeDilationUp`
  (params (Key :type "Key Structure"))
  ;[0.1506 0.5258 1 1 45] Input Handling - Time Dilation
  (:`Pressed`
    (`GameplayStatics.SetGlobalTimeDilation` (`KismetMathLibrary.FClamp` (+ (`GameplayStatics.GetGlobalTimeDilation`) (`self.Time Dilation Step`)) 0.0 2.0))))

(event `InputAction|TimeDilationDown`
  (params (Key :type "Key Structure"))
  ;[0.1506 0.5258 1 1 45] Input Handling - Time Dilation
  (:`Pressed`
    (`GameplayStatics.SetGlobalTimeDilation` (`KismetMathLibrary.FClamp` (- (`GameplayStatics.GetGlobalTimeDilation`) (`self.Time Dilation Step`)) 0.0 2.0))))

(event `InputAction|TimeDilationReset`
  (params (Key :type "Key Structure"))
  ;[0.1506 0.5258 1 1 45] Input Handling - Time Dilation
  (:`Pressed`
    (`GameplayStatics.SetGlobalTimeDilation` 1.0)))

(fn `Setup UI`
  (bind _returnvalue (`|CreateWidget` "/Game/VFXASandbox/UI/WBP_HiddenUI.WBP_HiddenUI_C" self))
  (bind _output_get (set `self.Hidden UI Widget` _returnvalue))
  (`UserWidget.AddToViewport` _output_get 0)
  (`Widget.SetVisibility` _output_get "Hidden")
  (bind _returnvalue_2 (`|CreateWidget` "/Game/VFXASandbox/UI/WBP_UI.WBP_UI_C" self))
  (bind _output_get_2 (set `self.UI Widget` _returnvalue_2))
  (`UserWidget.AddToViewport` _output_get_2 0))

(fn `UserConstructionScript`)