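; BP_ProjectileAbility is a projectile ability Blueprint whose only active logic handles the BPSpawnVFX event for casting effects.
; The event casts the supplied VFX asset to a Cascade particle system, falling back to a Niagara system if that fails.
; The effect spawns at the CastSocket on the mesh of player character 0, using that character's rotation.
; BeginPlay, overlap and Tick are disabled stubs.
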(event `self.BPSpawnVFX`
  (params (VFX :type "FXSystemAsset Object Reference"))
  (bind _returnvalue (`GameplayStatics.GetPlayerCharacter` 0))
  (bind _returnvalue_2 (`self.K2_GetActorRotation` _returnvalue))
  (bind _returnvalue_3 (`SceneComponent.GetSocketLocation` (`Character.Mesh` _returnvalue) "CastSocket"))
  (bind _asparticle_system (cast `ParticleSystem` VFX)
    (:`then`
      (`GameplayStatics.SpawnEmitterAtLocation` _asparticle_system _returnvalue_3 _returnvalue_2))
    (:`CastFailed`
      (`NiagaraFunctionLibrary.SpawnSystemAtLocation` (cast `NiagaraSystem` VFX :!pure true) _returnvalue_3 _returnvalue_2))))

(fn `UserConstructionScript`
  (`parent.UserConstructionScript`))